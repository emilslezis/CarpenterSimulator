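; Saw animation actor that plays the cut on a plank and swaps it for a triangle plank.
; On BeginPlay, the SawAnimation timeline moves and rotates the Saw component along a spline by distance.
; A Delay chained from the timeline's Update, rather than Finished, then destroys the found BP_Plank, the saw and the wood particles.
; It then spawns BP_TrianglePlank at the world origin.
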(event EventBeginPlay
  (bind _spline (Variables|Default|GetSpline))
  (bind _saw (Variables|Default|GetSaw))
  ;[1 1 1] Saw animation and spawn selected plank
  (bind _animation (Timeline|Saw%20animation PlayFromStart)
    (:Update
      (Transformation|SetWorldTransform _saw (Math|Transform|MakeTransform (Spline|GetLocationatDistanceAlongSpline _spline (* _animation (Spline|GetSplineLength _spline)) "World") (Spline|GetRotationatDistanceAlongSpline _spline (* _animation (Spline|GetSplineLength _spline)) "World") "0.125000,0.125000,0.125000") false false)
      (Utilities|FlowControl|Delay 5.0)
      (bind _returnvalue (Actor|GetActorOfClass "/Game/Blueprints/GetPlanks/BP_Plank.BP_Plank_C"))
      (Actor|DestroyActor _returnvalue)
      (Components|DestroyComponent _saw)
      (Components|DestroyComponent (Variables|Default|GetWoodParticles))
      (Game|SpawnActorfromClass "/Game/Blueprints/QuestPlanks/BP_TrianglePlank.BP_TrianglePlank_C" (Math|Transform|MakeTransform "0, 0, 0") "Undefined" 0 0))))

(fn ConstructionScript)