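; BP_GetPlanks is a quest interaction zone that lets the player place a plank on a table.
; Shape_Cube overlaps set an in-zone flag for any actor and toggle TakePlanks_Widget for the player character.
; Pressing F checks the interacting NPC's TookQuest and the zone flag, then spawns one BP_Plank at world origin and opens FirstQuestWidget with mouse cursor.
; TableHasPlank blocks repeat placement, with printed feedback.
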(event OnComponentBeginOverlap(Shape_Cube)
  (params (OverlappedComponent :type Primitive%20Component%20Object%20Reference) (OtherActor :type Actor%20Object%20Reference) (OtherComp :type Primitive%20Component%20Object%20Reference) (OtherBodyIndex :type Integer) (bFromSweep :type Boolean) (SweepResult :type Hit%20Result%20Structure%20%28by%20ref%29))
  (Variables|Default|SetIsInPlanksCollisionBox true)
  (Utilities|Casting|CastToThirdPersonCharacter OtherActor)
  ;[1 1 1] Put on/off press 'E' to take
  (bind _returnvalue (UserInterface|CreateWidget "/Game/Blueprints/GetPlanks/TakePlanks_Widget.TakePlanks_Widget_C"))
  (UserInterface|Viewport|AddtoViewport _returnvalue 0))

(event OnComponentEndOverlap(Shape_Cube)
  (params (OverlappedComponent :type Primitive%20Component%20Object%20Reference) (OtherActor :type Actor%20Object%20Reference) (OtherComp :type Primitive%20Component%20Object%20Reference) (OtherBodyIndex :type Integer))
  (Variables|Default|SetIsInPlanksCollisionBox false)
  (Utilities|Casting|CastToThirdPersonCharacter OtherActor)
  ;[1 1 1] Put on/off press 'E' to take
  (Widget|RemovefromParent (stale OnComponentBeginOverlap(Shape_Cube) _returnvalue)))

(event Input|KeyboardEvents|F
  (params (Key :type Key%20Structure :default "None"))
  (bind _returnvalue (Game|GetPlayerController 0))
  ;[1 1 1] Add plank on table
  (:Pressed
    (bind _asthird_person_character (Utilities|Casting|CastToThirdPersonCharacter (Game|GetPlayerCharacter 0)))
    (if (Variables|/Game/ThirdPersonBP/Blueprints/NPC.NPC_C|GetTookQuest (Variables|/Game/ThirdPersonBP/Blueprints/ThirdPersonCharacter.ThirdPersonCharacter_C|GetNPC%20To%20Interact _asthird_person_character))
      (if (Variables|Default|GetIsInPlanksCollisionBox)
        (if (Variables|Default|GetTableHasPlank)
          (Development|PrintString "Plank is already on table!")
          (else
            (Game|SpawnActorfromClass "/Game/Blueprints/GetPlanks/BP_Plank.BP_Plank_C" (Math|Transform|MakeTransform "0, 0, 0") "Undefined" 0 0)
            (Variables|Default|SetTableHasPlank true)
            (Development|PrintString "Plank placed on table.")
            (bind _returnvalue_2 (UserInterface|CreateWidget "/Game/Blueprints/HUD/FirstQuestWidget.FirstQuestWidget_C"))
            (UserInterface|Viewport|AddtoViewport _returnvalue_2 0)
            (Input|SetInputModeGameandUI _returnvalue 0 "DoNotLock" true)
            (Variables|/Script/Engine.PlayerController|SetbShowMouseCursor _returnvalue true))))
      (else
        (Development|PrintString "There is no active quest!")))))

(fn ConstructionScript)